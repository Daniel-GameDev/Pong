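; BP_Ball is the Pong ball, launched on a random diagonal at BeginPlay and moved every tick along Direction, scaled by Velocity and delta time.
; Movement is a world offset without sweep, so bounces come from the Collision component's begin-overlap event rather than physics.
; Walls report Side or Front through BPI_Walls to flip Y or X respectively, while hitting a BP_PlayerPlatform also flips X.
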(event `self.ReceiveBeginPlay`
  (`self.RandomDirection`))

(event `self.ReceiveTick`
  (params (DeltaSeconds :type "Float (single-precision)"))
  (set `self.Delta Seconds` DeltaSeconds)
  (`self.SphereDirectionOffset`))

(event `self.Collision.OnComponentBeginOverlap`
  (params (OverlappedComponent :type "PrimitiveComponent Object Reference") (OtherActor :type "Actor Object Reference") (OtherComp :type "PrimitiveComponent Object Reference") (OtherBodyIndex :type Integer) (bFromSweep :type Boolean) (SweepResult :type "HitResult Structure (by ref)"))
  (`self.Change Direction Based on Type` OtherActor))

(event `EventOffSet`)

(fn `Change Direction Based on Type`
  (params (Actor :type "Actor Object Reference"))
  (if (`KismetSystemLibrary.DoesImplementInterface` Actor "/Game/Pong/Blueprints/Common/BPI_Walls.BPI_Walls_C")
    (bind _walltype (message `/Game/Pong/Blueprints/Common/BPI_Walls.GetWallType` Actor))
    (switch `/Game/Pong/Blueprints/Common/EWallType` _walltype
      (:`NewEnumerator0`
        (`self.ChangeSide`))
      (:`NewEnumerator1`
        (`self.ChangeDirection` :!label _label)))
    (else
      (cast `/Game/Pong/Blueprints/Player/BP_PlayerPlatform` Actor)
      (goto _label))))

(fn `ChangeDirection`
  (bind (_direction_x _direction_y _direction_z) (`KismetMathLibrary.BreakVector` (`self.Direction`)))
  (set `self.Direction` (`KismetMathLibrary.MakeVector` (* _direction_x -1.0) _direction_y _direction_z)))

(fn `ChangeSide`
  (bind (_direction_x _direction_y _direction_z) (`KismetMathLibrary.BreakVector` (`self.Direction`)))
  (set `self.Direction` (`KismetMathLibrary.MakeVector` _direction_x (* _direction_y -1.0) _direction_z)))

(fn `RandomDirection`
  (bind _returnvalue (`KismetMathLibrary.RandomBool`))
  (bind _returnvalue_2 (`KismetMathLibrary.SelectFloat` 1.0 -1.0 _returnvalue))
  (if _returnvalue
    (set `self.Direction` (`KismetMathLibrary.MakeVector` _returnvalue_2 1.0))
    (else
      (set `self.Direction` (`KismetMathLibrary.MakeVector` _returnvalue_2 -1.0)))))

(fn `SphereDirectionOffset`
  (`self.K2_AddActorWorldOffset` (* (`self.Direction`) (* (`self.Delta Seconds`) (`self.Velocity`)))))

(fn `UserConstructionScript`)