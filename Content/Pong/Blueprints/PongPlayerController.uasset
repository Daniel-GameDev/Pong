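; Pong player controller that slides the controlled platform along world Y from the MoveRight input axis.
; On BeginPlay it negates Speed when the BP_PlayerPlatform's cube sits at positive X, reversing input for that side.
; Each move is tracked in DeltaLocation and applied through OffsetPlatform only if the total stays within MinRange and MaxRange.
; Input-mode switching nodes are present but never run.
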(event `self.ReceiveBeginPlay`
  (bind _asbp_player_platform (cast `/Game/Pong/Blueprints/BP_PlayerPlatform` (`self.K2_GetPawn`)))
  (bind _returnvalue_x (`KismetMathLibrary.BreakVector` (`SceneComponent.K2_GetComponentLocation` (`/Game/Pong/Blueprints/BP_PlayerPlatform.Cube` _asbp_player_platform))))
  (if (> _returnvalue_x 0.0)
    (set `self.Speed` (* (`self.Speed`) -1.0))))

(event `InputAxis|MoveRight`
  (params (AxisValue :type "Float (single-precision)"))
  (bind _returnvalue (* AxisValue (`self.Speed`)))
  (bind _returnvalue_2 (+ _returnvalue (`self.DeltaLocation`)))
  (if (!= AxisValue 0.0)
    (if (`KismetMathLibrary.InRange_FloatFloat` _returnvalue_2 (`self.MinRange`) (`self.MaxRange`))
      (set `self.DeltaLocation` _returnvalue_2)
      (`self.OffsetPlatform` (`Actor.RootComponent` (`self.K2_GetPawn`)) _returnvalue))))

(event `OffsetPlatform`
  (params (Platform :type "SceneComponent Object Reference") (DeltaY :type "Float (double-precision)"))
  (`SceneComponent.K2_AddWorldOffset` Platform (`KismetMathLibrary.MakeVector` 0.0 DeltaY) false false))

(fn `UserConstructionScript`)