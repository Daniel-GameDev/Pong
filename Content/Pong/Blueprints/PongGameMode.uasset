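; Game mode for two-player Pong that seats players on opposite sides, starts the match and respawns the ball after goals.
; ChoosePlayerStart maps each controller to its side's gate and camera, returning the PlayerStart tagged with that side.
; PostLogin sets the camera, binds the gate's end-overlap event and holds input until two players join, then spawns BP_Ball.
; AddScore only prints points without storing them, and several disconnected node chains remain.
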(event `self.ReceiveBeginPlay`)

(event `self.K2_PostLogin`
  (params (NewPlayer :type "PlayerController Object Reference"))
  (bind _as_pong_player_controller (`self.As Pong Player Controller`))
  (bind (_value _returnvalue) (`BlueprintMapLibrary.Map_Find` (`self.PlayerList`) _as_pong_player_controller))
  (bind _aspong_player_controller (cast `/Game/Pong/Blueprints/PongPlayerController` NewPlayer))
  (set `self.As Pong Player Controller` _aspong_player_controller)
  (`|ExecutionSequence`
    (:`then_0`
      (`WidgetBlueprintLibrary.SetInputMode_UIOnlyEx` _as_pong_player_controller null))
    (:`then_1`
      (if (`BlueprintMapLibrary.Map_Contains` (`self.PlayerList`) _as_pong_player_controller)
        (if _returnvalue
          (`PlayerController.SetViewTargetWithBlend` _as_pong_player_controller (`.Camera_12_4460CA304BDE5B523D7157AB40A89F15` (break `/Game/Pong/Blueprints/SPongPlayer` _value)) 0.0 "VTBlend_Linear" 0.0 false)
          (add `self.OnActorEndOverlap` (`.Gates_5_D12E06C64D7B5422F717CCAE168EA22A` (break `/Game/Pong/Blueprints/SPongPlayer` _value)) (`|CreateDelegate` :!event `AddScore`)))))
    (:`then_2`
      (if (< (`BlueprintMapLibrary.Map_Length` (`self.PlayerList`)) 2)
        (`KismetSystemLibrary.PrintString` "WAITING FOR SECOND PLAYER" true true (struct :`G` 0.66 :`B` 1.0 :`A` 1.0) 5.0)
        (else
          (`KismetSystemLibrary.PrintString` "Game Started.." true true (struct :`G` 0.66 :`B` 1.0 :`A` 1.0) 5.0)
          (`KismetSystemLibrary.Delay` 2.0)
          (bind _keys (`BlueprintMapLibrary.Map_Keys` (`self.PlayerList`)))
          (for _array_element _keys
            (`WidgetBlueprintLibrary.SetInputMode_GameOnly` _array_element))
          (`self.SpawnBall`))))))

(event `SpawnBall`
  (`|SpawnActorFromClass` "/Game/Pong/Blueprints/BP_Ball.BP_Ball_C" (`KismetMathLibrary.MakeTransform` (`self.Spawn Transform Location`)) "Undefined" "OverrideRootScale" null null))

(event `self.K2_OnLogout`
  (params (ExitingController :type "Controller Object Reference")))

(event `AddScore` :!signature `self.OnActorEndOverlap`
  (params (OverlappedActor :type "Actor Object Reference") (OtherActor :type "Actor Object Reference"))
  (bind _asbp_gates (cast `/Game/Pong/Blueprints/BP_Gates` OverlappedActor))
  (`KismetSystemLibrary.PrintString` "BallWasDestroyed" true true (struct :`R` 1.0 :`B` 0.08483 :`A` 1.0) 5.0)
  (switch `/Game/Pong/Blueprints/EPlayerSide` (`/Game/Pong/Blueprints/BP_Gates.GatesSide` _asbp_gates)
    (:`NewEnumerator0`
      (`KismetSystemLibrary.PrintString` "Brown +1" true true (struct :`R` 1.0 :`B` 0.08483 :`A` 1.0) 5.0))
    (:`NewEnumerator1`
      (`KismetSystemLibrary.PrintString` "Green +1" true true (struct :`R` 1.0 :`B` 0.08483 :`A` 1.0) 5.0)))
  (`KismetSystemLibrary.Delay` 2.0)
  (`self.SpawnBall`))

(event `Update_PlayerList`)

(fn `ChoosePlayerStart`
  (params (Player :type "Controller Object Reference"))
  (returns (ReturnValue :type "Actor Object Reference"))
  (locals (Local_Side :type "/Game/Pong/Blueprints/EPlayerSide Enum" :default "NewEnumerator0"))
  (bind _aspong_player_controller (cast `/Game/Pong/Blueprints/PongPlayerController` Player))
  (if (== (`BlueprintMapLibrary.Map_Length` (`self.PlayerList`)) 0)
    (bind _output_get (set `local.Local_Side` "NewEnumerator1"))
    (bind _playerstruct (`self.SetupPlayerData` _output_get))
    (`BlueprintMapLibrary.Map_Add` (`self.PlayerList`) _aspong_player_controller _playerstruct)
    (else
      (bind _output_get_2 (set `local.Local_Side` "NewEnumerator0"))
      (bind _playerstruct_2 (`self.SetupPlayerData` _output_get_2))
      (`BlueprintMapLibrary.Map_Add` (`self.PlayerList`) _aspong_player_controller _playerstruct_2)))
  (bind _outactors (`GameplayStatics.GetAllActorsOfClass` "/Script/Engine.PlayerStart"))
  (for _array_element _outactors
    (if (== (`PlayerStart.PlayerStartTag` _array_element) (`KismetStringLibrary.Conv_StringToName` (`|GetEnumeratorNameAsString` (`local.Local_Side`))))
      (return _array_element))))

(fn `SetupPlayerData`
  (params (Side :type "/Game/Pong/Blueprints/EPlayerSide Enum" :default "NewEnumerator0"))
  (returns (PlayerStruct :type "/Game/Pong/Blueprints/SPongPlayer Structure"))
  (locals (Local_Gates :type "/Game/Pong/Blueprints/BP_Gates Object Reference") (Local_Camera :type "/Game/Pong/Blueprints/BP_PlayerCamera Object Reference"))
  (bind _side (`local.Side`))
  (bind _outactors (`GameplayStatics.GetAllActorsOfClass` "/Game/Pong/Blueprints/BP_Gates.BP_Gates_C"))
  (for _array_element _outactors
    (if (`|EnumEquality` (`/Game/Pong/Blueprints/BP_Gates.GatesSide` _array_element) _side)
      (set `local.Local_Gates` _array_element)
      (bind _outactors_2 (`GameplayStatics.GetAllActorsOfClass` "/Game/Pong/Blueprints/BP_PlayerCamera.BP_PlayerCamera_C"))
      (for _array_element_2 _outactors_2
        (if (`|EnumEquality` (`/Game/Pong/Blueprints/BP_PlayerCamera.CameraSide` _array_element_2) _side)
          (set `local.Local_Camera` _array_element_2)
          (return (make `/Game/Pong/Blueprints/SPongPlayer` (`local.Side`) (`local.Local_Gates`) (`local.Local_Camera`))))))))

(fn `UserConstructionScript`)