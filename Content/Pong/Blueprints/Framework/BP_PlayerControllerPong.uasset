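; Player controller for the Pong game that manages its UI widgets and input mode.
; Custom events create the score widget and the game-start widget and add them to the viewport.
; UpdateScore forwards a side to the stored score widget's AddScore.
; ControlInputClient switches between game-only and UI-only input.
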(event `UpdateScore`
  (params (Side :type "EArenaSides Enum" :default "EAS_RightSide"))
  (bind _aswbp_score (cast `/Game/Pong/Blueprints/UI/WBP_Score` (`self.ScoretWidget`)))
  (`/Game/Pong/Blueprints/UI/WBP_Score.AddScore` _aswbp_score Side))

(event `CreateScore`
  (bind _returnvalue (`|CreateWidget` "/Game/Pong/Blueprints/UI/WBP_Score.WBP_Score_C" self))
  (bind _output_get (set `self.ScoretWidget` _returnvalue))
  (`UserWidget.AddToViewport` _output_get 0))

(event `CreateWidgetBeginGame`
  (bind _returnvalue (`|CreateWidget` "/Game/Pong/Blueprints/UI/WBP_GameStart.WBP_GameStart_C" self))
  (`UserWidget.AddToViewport` _returnvalue 0))

(event `ControlInputClient`
  (params (Enable :type Boolean))
  (if Enable
    (`WidgetBlueprintLibrary.SetInputMode_GameOnly` self)
    (else
      (`WidgetBlueprintLibrary.SetInputMode_UIOnlyEx` self null))))

(fn `UserConstructionScript`)