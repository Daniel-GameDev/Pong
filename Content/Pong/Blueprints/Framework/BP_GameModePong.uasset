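; Game mode for Pong that holds the match until two players have joined, then runs the start, ball spawning and scoring flow.
; On login it disables the newcomer's input and either shows a wait widget to the first player or starts the begin-game widgets.
; The first player's countdown widget triggers StartGame, which enables input, creates score displays and spawns the ball.
; AddScore updates the given controller's score and respawns the ball after a delay.
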(event `self.K2_PostLogin`
  (params (NewPlayer :type "PlayerController Object Reference"))
  (bind _wait (`self.Wait`))
  (`parent.K2_PostLogin` NewPlayer)
  (bind _asbp_player_controller_pong (cast `/Game/Pong/Blueprints/Framework/BP_PlayerControllerPong` NewPlayer))
  (`/Game/Pong/Blueprints/Framework/BP_PlayerControllerPong.ControlInputClient` _asbp_player_controller_pong false)
  (if (< (`BlueprintMapLibrary.Map_Length` (`self.PongPlayers`)) 2)
    (bind _keys (`BlueprintMapLibrary.Map_Keys` (`self.PongPlayers`)))
    (bind _returnvalue (`|CreateWidget` "/Game/Pong/Blueprints/UI/WBP_Wait.WBP_Wait_C" (`|GetArrayItem` _keys)))
    (bind _output_get (set `self.Wait` _returnvalue))
    (`UserWidget.AddToViewport` _output_get 0)
    (else
      (`/Engine/EditorBlueprintResources/StandardMacros.IsValid` _wait
        (:`Is Valid`
          (`Widget.RemoveFromParent` _wait))
        (:`Is Not Valid`
          _))
      (bind _keys_2 (`BlueprintMapLibrary.Map_Keys` (`self.PongPlayers`)))
      (for (_array_element _array_index) _keys_2
        (if (== _array_index 0)
          (bind _returnvalue_2 (`|CreateWidget` "/Game/Pong/Blueprints/UI/WBP_GameStart.WBP_GameStart_C" _array_element))
          (`UserWidget.AddToViewport` _returnvalue_2 0)
          (add `/Game/Pong/Blueprints/UI/WBP_GameStart.TimeFinished` _returnvalue_2 (delegate `StartGame`))
          (else
            (bind _asbp_player_controller_pong_2 (cast `/Game/Pong/Blueprints/Framework/BP_PlayerControllerPong` _array_element))
            (`/Game/Pong/Blueprints/Framework/BP_PlayerControllerPong.CreateWidgetBeginGame` _asbp_player_controller_pong_2)))))))

(event `StartGame`
  (bind _keys (`BlueprintMapLibrary.Map_Keys` (`self.PongPlayers`)))
  (for _array_element _keys
    (bind _asbp_player_controller_pong (cast `/Game/Pong/Blueprints/Framework/BP_PlayerControllerPong` _array_element))
    (`/Game/Pong/Blueprints/Framework/BP_PlayerControllerPong.ControlInputClient` _asbp_player_controller_pong true)
    (`/Game/Pong/Blueprints/Framework/BP_PlayerControllerPong.CreateScore` _asbp_player_controller_pong))
  (`self.SpawnBall`))

(event `self.AddScore`
  (params (PongPlayer :type "PlayerController Object Reference") (PlayerSide :type "EArenaSides Enum" :default "EAS_RightSide"))
  (bind _asbp_player_controller_pong (cast `/Game/Pong/Blueprints/Framework/BP_PlayerControllerPong` PongPlayer))
  (`/Game/Pong/Blueprints/Framework/BP_PlayerControllerPong.UpdateScore` _asbp_player_controller_pong PlayerSide)
  (`KismetSystemLibrary.Delay` (`self.BallSpawnTimeDelay`))
  (`self.SpawnBall`))

(fn `ChoosePlayerStart`
  (params (Player :type "Controller Object Reference"))
  (returns (ReturnValue :type "Actor Object Reference"))
  (bind _asbp_player_controller_pong (cast `/Game/Pong/Blueprints/Framework/BP_PlayerControllerPong` Player))
  (bind _returnvalue (`self.GetStartPoint` _asbp_player_controller_pong))
  (return _returnvalue))

(fn `UserConstructionScript`)