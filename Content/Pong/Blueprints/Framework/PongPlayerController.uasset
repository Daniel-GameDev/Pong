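; Player controller for Pong that moves the player's platform sideways and manages that player's UI.
; MoveRight input offsets the controlled pawn along Y while an accumulated delta stays in range, with speed negated at BeginPlay for a platform at positive X.
; Custom events create the score and game-start widgets, forward scoring by side to the score widget, and switch input between game-only and UI-only modes.
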(event `UpdateScore`
  (params (Side :type "/Game/Pong/Blueprints/Common/ESide Enum" :default "NewEnumerator0"))
  (`/Game/Pong/Blueprints/UI/WBP_Score.AddScore` (`self.Score`) Side))

(event `CreateScore`
  (bind _returnvalue (`|CreateWidget` "/Game/Pong/Blueprints/UI/WBP_Score.WBP_Score_C" self))
  (bind _output_get (set `self.Score` _returnvalue))
  (`UserWidget.AddToViewport` _output_get 0))

(event `CreateWidgetBeginGame`
  (bind _returnvalue (`|CreateWidget` "/Game/Pong/Blueprints/UI/WBP_GameStart.WBP_GameStart_C" self))
  (`UserWidget.AddToViewport` _returnvalue 0))

(event `ControlInputClient`
  (params (Enable :type Boolean))
  (if Enable
    (`WidgetBlueprintLibrary.SetInputMode_GameOnly` self)
    (else
      (`WidgetBlueprintLibrary.SetInputMode_UIOnlyEx` self null))))

(event `self.ReceiveBeginPlay`
  (bind _asbp_player_platform (cast `/Game/Pong/Blueprints/Player/BP_PlayerPlatform` (`self.K2_GetPawn`)))
  (bind _returnvalue_x (`KismetMathLibrary.BreakVector` (`SceneComponent.K2_GetComponentLocation` (`/Game/Pong/Blueprints/Player/BP_PlayerPlatform.Cube` _asbp_player_platform))))
  (if (> _returnvalue_x 0.0)
    (set `self.Speed` (* (`self.Speed`) -1.0))))

(event `InputAxis|MoveRight`
  (params (AxisValue :type "Float (single-precision)"))
  (bind _returnvalue (* AxisValue (`self.Speed`)))
  (bind _returnvalue_2 (+ _returnvalue (`self.DeltaLocation`)))
  (if (!= AxisValue 0.0)
    (if (`KismetMathLibrary.InRange_FloatFloat` _returnvalue_2 (`self.MinRange`) (`self.MaxRange`))
      (set `self.DeltaLocation` _returnvalue_2)
      (`self.OffsetPlatform` (`Actor.RootComponent` (`self.K2_GetPawn`)) _returnvalue))))

(event `OffsetPlatform`
  (params (Platform :type "SceneComponent Object Reference") (DeltaY :type "Float (double-precision)"))
  (`SceneComponent.K2_AddWorldOffset` Platform (`KismetMathLibrary.MakeVector` 0.0 DeltaY) false false))

(fn `UserConstructionScript`)