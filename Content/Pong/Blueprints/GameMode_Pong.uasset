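; Game mode for a two-player Pong game that assigns each joining player a side of the arena.
; ChoosePlayerStart gives the first controller one side and later ones the other, stores that side's gates and camera in PlayerList, and returns the PlayerStart tagged with the side's name.
; PostLogin then blends the player's view to the stored camera.
; Several leftover list-update and camera chains are disconnected and never run.
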(event `self.ReceiveBeginPlay`)

(event `self.K2_PostLogin`
  (params (NewPlayer :type "PlayerController Object Reference"))
  (bind _asplayer_controller_pong (cast `/Game/Pong/Blueprints/PlayerController_Pong` NewPlayer))
  (if (`BlueprintMapLibrary.Map_Contains` (`self.PlayerList`) _asplayer_controller_pong)
    (if true
      (bind _value (`BlueprintMapLibrary.Map_Find` (`self.PlayerList`) _asplayer_controller_pong))
      (set `self.NewVar_0` (break `/Game/Pong/Blueprints/SPongPlayer` _value))
      (set `self.Camera Side` (`/Game/Pong/Blueprints/BP_PlayerCamera.CameraSide` (`.Camera_12_4460CA304BDE5B523D7157AB40A89F15` (break `/Game/Pong/Blueprints/SPongPlayer` _value))))
      (`PlayerController.SetViewTargetWithBlend` _asplayer_controller_pong (`.Camera_12_4460CA304BDE5B523D7157AB40A89F15` (break `/Game/Pong/Blueprints/SPongPlayer` _value)) 0.0 "VTBlend_Linear" 0.0 false))))

(event `self.K2_OnLogout`
  (params (ExitingController :type "Controller Object Reference")))

(event `Update_PlayerList`)

(fn `ChoosePlayerStart`
  (params (Player :type "Controller Object Reference"))
  (returns (ReturnValue :type "Actor Object Reference"))
  (locals (Local_Side :type "/Game/Pong/Blueprints/EPlayerSide Enum" :default "NewEnumerator0"))
  (bind _asplayer_controller_pong (cast `/Game/Pong/Blueprints/PlayerController_Pong` Player))
  (if (== (`BlueprintMapLibrary.Map_Length` (`self.PlayerList`)) 0)
    (bind _output_get (set `local.Local_Side` "NewEnumerator1"))
    (bind _playerstruct (`self.SetupPlayerData` _output_get))
    (`BlueprintMapLibrary.Map_Add` (`self.PlayerList`) _asplayer_controller_pong _playerstruct)
    (else
      (bind _output_get_2 (set `local.Local_Side` "NewEnumerator0"))
      (bind _playerstruct_2 (`self.SetupPlayerData` _output_get_2))
      (`BlueprintMapLibrary.Map_Add` (`self.PlayerList`) _asplayer_controller_pong _playerstruct_2)))
  (bind _outactors (`GameplayStatics.GetAllActorsOfClass` "/Script/Engine.PlayerStart"))
  (for _array_element _outactors
    (if (== (`PlayerStart.PlayerStartTag` _array_element) (`KismetStringLibrary.Conv_StringToName` (`|GetEnumeratorNameAsString` (`local.Local_Side`))))
      (return _array_element))))

(fn `SetupPlayerData`
  (params (Side :type "/Game/Pong/Blueprints/EPlayerSide Enum" :default "NewEnumerator0"))
  (returns (PlayerStruct :type "/Game/Pong/Blueprints/SPongPlayer Structure"))
  (locals (Local_Gates :type "/Game/Pong/Blueprints/BP_Gates Object Reference") (Local_Camera :type "/Game/Pong/Blueprints/BP_PlayerCamera Object Reference"))
  (bind _side (`local.Side`))
  (bind _outactors (`GameplayStatics.GetAllActorsOfClass` "/Game/Pong/Blueprints/BP_Gates.BP_Gates_C"))
  (for _array_element _outactors
    (if (`|EnumEquality` (`/Game/Pong/Blueprints/BP_Gates.GatesSide` _array_element) _side)
      (set `local.Local_Gates` _array_element)
      (bind _outactors_2 (`GameplayStatics.GetAllActorsOfClass` "/Game/Pong/Blueprints/BP_PlayerCamera.BP_PlayerCamera_C"))
      (for _array_element_2 _outactors_2
        (if (`|EnumEquality` (`/Game/Pong/Blueprints/BP_PlayerCamera.CameraSide` _array_element_2) _side)
          (set `local.Local_Camera` _array_element_2)
          (return (make `/Game/Pong/Blueprints/SPongPlayer` (`local.Side`) (`local.Local_Gates`) (`local.Local_Camera`))))))))

(fn `UserConstructionScript`)