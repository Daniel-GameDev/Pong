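; Player controller for Pong that slides the controlled pawn sideways along world Y from the MoveRight axis.
; BeginPlay looks up the player's match index with an empty match ID and reverses Speed when the result is -1.
; Each non-zero input adds a Speed-scaled offset to the pawn's root, tracking accumulated DeltaLocation and ignoring steps that would leave the MinRange to MaxRange bounds.
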(event `self.ReceiveBeginPlay`
  (bind _playerindex (`TurnBasedBlueprintLibrary.GetMyPlayerIndex` self))
  (bind _output_get (set `self.Player Index` _playerindex))
  (if (== _output_get -1)
    (set `self.Speed` (* (`self.Speed`) -1.0))))

(event `InputAxis|MoveRight`
  (params (AxisValue :type "Float (single-precision)"))
  (bind _returnvalue (* AxisValue (`self.Speed`)))
  (bind _returnvalue_2 (+ _returnvalue (`self.DeltaLocation`)))
  (if (!= AxisValue 0.0)
    (if (`KismetMathLibrary.InRange_FloatFloat` _returnvalue_2 (`self.MinRange`) (`self.MaxRange`))
      (set `self.DeltaLocation` _returnvalue_2)
      (`SceneComponent.K2_AddWorldOffset` (`Actor.RootComponent` (`self.K2_GetPawn`)) (`KismetMathLibrary.MakeVector` 0.0 _returnvalue) false false))))

(fn `UserConstructionScript`)